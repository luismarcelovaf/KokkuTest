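; Pong game state that sets up each match's view and spawns client-side stand-ins for networked actors.
; On BeginPlay it sets game-only input without a cursor and points the player's view at the level's single CameraActor.
; On clients only, it spawns a FakeBar at the left Bar's transform, storing it on the PongController.
; It also spawns a FakeBall at the Ball's transform, linked to the real Ball.
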(event EventBeginPlay
  (bind _returnvalue (Game|GetPlayerController 0))
  (bind _returnvalue_2 (Game|GetPlayerController 0))
  ;[1 1 1] Attaches Camera
  (Variables|/Script/Engine.PlayerController|SetbShowMouseCursor _returnvalue false)
  (Input|SetInputModeGameOnly _returnvalue)
  (bind _returnvalue_3 (Actor|GetActorOfClass "/Script/Engine.CameraActor")) ; Note: Our level cannot have more than one camera using this
  (Game|Player|SetViewTargetwithBlend _returnvalue _returnvalue_3 0.0 "VTBlend_Linear" 0.0 false)
  ;[1 1 1] Spawn Client Bar
  (Utilities|IsServer
    (:Client
      (bind _outactors (Actor|GetAllActorsOfClass "/Game/Blueprints/Pawns/Bar.Bar_C"))
      (for _array_element _outactors
        (switch Utilities|FlowControl|Switch|SwitchonBarType (Variables|/Game/Blueprints/Pawns/Bar.Bar_C|GetBarType _array_element)
          (:NewEnumerator0
            (bind _returnvalue_4 (Game|SpawnActorfromClass "/Game/Blueprints/Client/FakeBar.FakeBar_C" (Transformation|GetActorTransform _array_element) "Undefined" _returnvalue_2 0)) ; Upon enter match, spawn dummy player bar
            (Variables|/Game/Blueprints/PongController.PongController_C|SetPlayerFakeBar (.AsPong%20Controller (Utilities|Casting|CastToPongController _returnvalue_2)) _returnvalue_4)
            ;[1 1 1] Spawn Client Ball
            (bind _returnvalue_5 (Actor|GetActorOfClass "/Game/Blueprints/Actors/Ball.Ball_C"))
            (Game|SpawnActorfromClass "/Game/Blueprints/Client/FakeBall.FakeBall_C" (Transformation|GetActorTransform _returnvalue_5) "Undefined" (Game|GetPlayerController 0) _returnvalue_5 0) ; Upon enter match, spawn dummy ball
          ))))))

(fn ConstructionScript)