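; Pong-style ball actor that moves by physics velocity and bounces off bars and boundaries.
; It launches with a randomized horizontal and vertical velocity scaled by BallSpeed on BeginPlay.
; Overlapping a Bar mirrors X and speeds it up slightly, while a Boundary mirrors Y.
; On clients the replicated "real" ball turns green and starts hidden, with events to toggle its visibility there only.
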(event OnComponentBeginOverlap(StaticMesh)
  (params (OverlappedComponent :type Primitive%20Component%20Object%20Reference) (OtherActor :type Actor%20Object%20Reference) (OtherComp :type Primitive%20Component%20Object%20Reference) (OtherBodyIndex :type Integer) (bFromSweep :type Boolean) (SweepResult :type Hit%20Result%20Structure%20%28by%20ref%29))
  ;[1 1 1] Bar Hit
  (Utilities|Casting|CastToBar OtherActor
    (:then
      (bind _returnvalue (Physics|GetPhysicsLinearVelocity (Variables|Default|GetStaticMesh) "None"))
      (Physics|SetPhysicsLinearVelocity (Variables|Default|GetStaticMesh) (Math|Vector|MakeVector (* (.X (Math|Vector|BreakVector _returnvalue)) -1.05) (.Y (Math|Vector|BreakVector _returnvalue)) 0.0) false "None"))
    (:CastFailed
      ;[1 1 1] Boundary Hit
      (Utilities|Casting|CastToBoundary OtherActor)
      (bind _returnvalue_2 (Physics|GetPhysicsLinearVelocity (Variables|Default|GetStaticMesh) "None")) ; Hitting boundary does not change direction
      (Physics|SetPhysicsLinearVelocity (Variables|Default|GetStaticMesh) (Math|Vector|MakeVector (.X (Math|Vector|BreakVector _returnvalue_2)) (* (.Y (Math|Vector|BreakVector _returnvalue_2)) -1.0) 0.0) false "None"))))

(event Custom|SetRandomVelocity
  (bind _returnvalue (Math|Random|RandomFloatinRange 0.5 1.0))
  (bind _returnvalue_2 (- _returnvalue 1.0))
  ;[1 1 1] Sets random velocity
  (Physics|SetPhysicsLinearVelocity (Variables|Default|GetStaticMesh) (* (Math|Vector|MakeVector (Math|Float|SelectFloat _returnvalue (* _returnvalue -1.0) (Math|Random|RandomBool)) (Math|Float|SelectFloat _returnvalue_2 (* _returnvalue_2 -1.0) (Math|Random|RandomBool)) 0.0) (Variables|Default|GetBallSpeed)) false "None"))

(event Custom|DisableVisibility
  ;[1 1 1] Visibility
  (Networking|SwitchHasAuthority
    (:Remote
      (Rendering|SetVisibility (Variables|Default|GetStaticMesh) false false))))

(event Custom|EnableVisibility
  ;[1 1 1] Visibility
  (Networking|SwitchHasAuthority
    (:Remote
      (Rendering|SetVisibility (Variables|Default|GetStaticMesh) true false))))

(event EventBeginPlay
  ;[1 1 1] Initialize Velocity
  (CallFunction|SetRandomVelocity)
  ;[1 1 1] Set Material Only for Client's Real Ball
  (Networking|SwitchHasAuthority
    (:Remote
      (Rendering|Material|SetMaterial (Variables|Default|GetStaticMesh) 0 "/Game/Materials/BasicGreen.BasicGreen")
      (Rendering|SetVisibility (Variables|Default|GetStaticMesh) false false))))

(fn ConstructionScript)