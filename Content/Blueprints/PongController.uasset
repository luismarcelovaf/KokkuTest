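; Player controller for networked Pong that turns Up/Down input into paddle movement, with client-side fake-bar prediction.
; Input drives PlayerBar, while clients also move PlayerFakeBar and, on key release, sync the real bar to its location.
; Debug keys toggle real bar and ball visibility on clients and simulate packet lag through console commands.
; GetBarOfType is a helper that finds a Bar actor by type.
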(event Custom|SyncBar
  ;[1 1 1] Syncs Real Bar Position
  (Default|Sync (Variables|Default|GetPlayerBar) (Transformation|GetActorLocation (Variables|Default|GetPlayerFakeBar))))

(event Custom|ToggleDebug
  ;[1 1 1] Toggle Debug Mode
  (Utilities|FlowControl|FlipFlop
    (:A
      (Default|EnableVisibility (Variables|Default|GetBall))
      (Development|PrintString "Debug Activated"))
    (:B
      (Default|DisableVisibility (Variables|Default|GetBall))
      (Development|PrintString "Debug Deactivated"))))

(event Input|KeyboardEvents|Up
  (params (Key :type Key%20Structure :default "None"))
  (bind _playerfakebar (Variables|Default|GetPlayerFakeBar))
  (bind _playerbar (Variables|Default|GetPlayerBar))
  ;[1 1 1] Bar Movement Control
  (:Pressed
    (Default|MoveUp _playerbar)
    (Utilities|IsServer
      (:Client
        (Default|MoveUp _playerfakebar))))
  (:Released
    (Default|MoveStop _playerbar)
    (Utilities|IsServer
      (:Client
        (Default|MoveStop _playerfakebar)
        (CallFunction|SyncBar)))))

(event Input|KeyboardEvents|Down
  (params (Key :type Key%20Structure :default "None"))
  (bind _playerfakebar (Variables|Default|GetPlayerFakeBar))
  (bind _playerbar (Variables|Default|GetPlayerBar))
  ;[1 1 1] Bar Movement Control
  (:Pressed
    (Default|MoveDown _playerbar)
    (Utilities|IsServer
      (:Client
        (Default|MoveDown _playerfakebar))))
  (:Released
    (Default|MoveStop _playerbar)
    (Utilities|IsServer
      (:Client
        (Default|MoveStop _playerfakebar)
        (CallFunction|SyncBar)))))

(event Input|KeyboardEvents|D
  (params (Key :type Key%20Structure :default "None"))
  ;[1 1 1] Toggle Debug Mode
  (:Pressed
    (Utilities|IsServer
      (:Client
        (Utilities|FlowControl|FlipFlop
          (:A
            (Default|EnableVisibility (Variables|Default|GetPlayerBar)))
          (:B
            (Default|DisableVisibility (Variables|Default|GetPlayerBar))))
        (CallFunction|ToggleDebug) ; Left Bar is Owned by client but Ball is Owned by Server
      ))))

(event Input|KeyboardEvents|F
  (params (Key :type Key%20Structure :default "None"))
  ;[1 1 1] Toggle Latency Mode
  (:Pressed
    (Utilities|FlowControl|FlipFlop
      (:A
        (Development|ExecuteConsoleCommand "Net PktLag=150?Net PktLagVariance=100" 0)
        (Development|PrintString "Latency Activated"))
      (:B
        (Development|ExecuteConsoleCommand "Net PktLag=0?Net PktLagVariance=0" 0)
        (Development|PrintString "Latency Deactivated")))))

(fn ConstructionScript)

(fn GetBarOfType
  (params (BarType :type BarType%20Enum :default "NewEnumerator0"))
  (bind _outactors (Actor|GetAllActorsOfClass "/Game/Blueprints/Pawns/Bar.Bar_C"))
  (for _array_element _outactors
    (if (Utilities|Enum|Equal(Enum) (Variables|/Game/Blueprints/Pawns/Bar.Bar_C|GetBarType _array_element) BarType)
      (return _array_element))))