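; Game mode for a multiplayer Pong game that pauses on begin play and logout, and unpauses when a player logs in.
; On login it gives the new controller the Ball and left Bar, with ownership, and assigns the right Bar to player controller 0.
; Logout returns the leaving player's bar ownership to the game mode.
; ReadyToStartMatch always returns true, leaving its MaxNumPlayers check (parsed from the options string) disconnected.
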(event EventBeginPlay
  ;[1 1 1] Updates Number of Players Variable
  (Variables|Default|SetMaxNumPlayers (Math|Conversions|ToInteger(Byte) (Class|GameplayStatics|ParseOption (Variables|Default|GetOptionsString) "MaxNumPlayers")))
  (Game|SetGamePaused true)
  (Variables|Default|SetGameReady false))

(event EventPostLogin
  (params (NewPlayer :type Player%20Controller%20Object%20Reference))
  ;[1 1 1] Player Login
  (Variables|Default|SetController NewPlayer)
  (Game|SetGamePaused false)
  (Variables|Default|SetGameReady true)
  (Development|PrintString (Utilities|String|Append "Player Connected: " (Utilities|GetDisplayName NewPlayer)))
  ;[1 1 1] Initializes Ball
  (bind _returnvalue (Actor|GetActorOfClass "/Game/Blueprints/Actors/Ball.Ball_C"))
  (Variables|/Game/Blueprints/PongController.PongController_C|SetBall (.AsPong%20Controller (Utilities|Casting|CastToPongController (Variables|Default|GetController))) _returnvalue)
  ;[1 1 1] Initializes Bars
  (bind _outactors (Actor|GetAllActorsOfClass "/Game/Blueprints/Pawns/Bar.Bar_C"))
  (for _array_element _outactors
    (switch Utilities|FlowControl|Switch|SwitchonBarType (Variables|/Game/Blueprints/Pawns/Bar.Bar_C|GetBarType _array_element)
      (:NewEnumerator0
        (bind _output_get (Variables|/Game/Blueprints/PongController.PongController_C|SetPlayerBar (.AsPong%20Controller (Utilities|Casting|CastToPongController (Variables|Default|GetController))) _array_element))
        (Actor|SetOwner _output_get (.AsPong%20Controller (Utilities|Casting|CastToPongController (Variables|Default|GetController)))))
      (:NewEnumerator1
        (Variables|/Game/Blueprints/PongController.PongController_C|SetPlayerBar (.AsPong%20Controller (Utilities|Casting|CastToPongController (Game|GetPlayerController 0))) _array_element)))))

(event EventOnLogout
  (params (ExitingController :type Controller%20Object%20Reference))
  ;[1 1 1] Player Logout
  (Game|SetGamePaused true)
  (Variables|Default|SetGameReady false)
  (Actor|SetOwner (Variables|/Game/Blueprints/PongController.PongController_C|GetPlayerBar (.AsPong%20Controller (Utilities|Casting|CastToPongController ExitingController))) self))

(fn ConstructionScript)

(fn ReadytoStartMatch
  (return true))