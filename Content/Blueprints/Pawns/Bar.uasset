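; Networked paddle pawn that moves along the Y axis at a set speed from up, down and stop input events.
; Tick applies the input as physics velocity, blocking motion toward any Boundary its mesh overlaps.
; The left bar, treated as the client's, eases toward the last synced position while idle to correct drift.
; On clients it also gets a green material and starts hidden until visibility is enabled.
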(event OnComponentBeginOverlap(StaticMesh)
  (params (OverlappedComponent :type Primitive%20Component%20Object%20Reference) (OtherActor :type Actor%20Object%20Reference) (OtherComp :type Primitive%20Component%20Object%20Reference) (OtherBodyIndex :type Integer) (bFromSweep :type Boolean) (SweepResult :type Hit%20Result%20Structure%20%28by%20ref%29))
  ;[1 1 1] Start colliding
  (bind _asboundary (Utilities|Casting|CastToBoundary OtherActor))
  (switch Utilities|FlowControl|Switch|SwitchonBoundaryType (Variables|/Game/Blueprints/Actors/Boundary.Boundary_C|GetBoundaryType _asboundary)
    (:NewEnumerator0
      (Variables|Default|SetCollidingUp true))
    (:NewEnumerator1
      (Variables|Default|SetCollidingDown true))))

(event OnComponentEndOverlap(StaticMesh)
  (params (OverlappedComponent :type Primitive%20Component%20Object%20Reference) (OtherActor :type Actor%20Object%20Reference) (OtherComp :type Primitive%20Component%20Object%20Reference) (OtherBodyIndex :type Integer))
  ;[1 1 1] End colliding
  (bind _asboundary (Utilities|Casting|CastToBoundary OtherActor))
  (switch Utilities|FlowControl|Switch|SwitchonBoundaryType (Variables|/Game/Blueprints/Actors/Boundary.Boundary_C|GetBoundaryType _asboundary)
    (:NewEnumerator0
      (Variables|Default|SetCollidingUp false))
    (:NewEnumerator1
      (Variables|Default|SetCollidingDown false))))

(event Custom|MoveUp
  ;[1 1 1] Inputs
  (Variables|Default|SetMovementVector (* (Math|Vector|MakeVector 0.0 -1.0 0.0) (Variables|Default|GetBarSpeed))))

(event Custom|MoveDown
  ;[1 1 1] Inputs
  (Variables|Default|SetMovementVector (* (Math|Vector|MakeVector 0.0 1.0 0.0) (Variables|Default|GetBarSpeed))))

(event Custom|MoveStop
  ;[1 1 1] Inputs
  (Variables|Default|SetMovementVector "0, 0, 0"))

(event Custom|DisableVisibility
  ;[1 1 1] Visibility
  (switch Utilities|FlowControl|Switch|SwitchonBarType (Variables|Default|GetBarType)
    (:NewEnumerator0
      (Rendering|SetVisibility (Variables|Default|GetStaticMesh) false false))))

(event Custom|EnableVisibility
  ;[1 1 1] Visibility
  (switch Utilities|FlowControl|Switch|SwitchonBarType (Variables|Default|GetBarType)
    (:NewEnumerator0
      (Rendering|SetVisibility (Variables|Default|GetStaticMesh) true false))))

(event Custom|Sync
  (params (Position :type Vector))
  ;[1 1 1] Timed Sync Position
  (Variables|Default|SetLastKnownPosition Position))

(event EventTick
  (params (DeltaSeconds :type Float%20%28single-precision%29))
  (bind _returnvalue (Transformation|GetActorLocation))
  (bind _collidingup (Variables|Default|GetCollidingUp))
  (bind _collidingdown (Variables|Default|GetCollidingDown))
  (bind _lastknownposition (Variables|Default|GetLastKnownPosition))
  (bind _movementvector (Variables|Default|GetMovementVector))
  (bind (_x _y) (Math|Vector|BreakVector _movementvector))
  (bind _returnvalue_2 (Math|Interpolation|VInterpTo _returnvalue _lastknownposition DeltaSeconds 5.0))
  (bind _returnvalue_3 (Math|Float|Max(Float) _y 0.0))
  (bind _returnvalue_4 (Math|Vector|MakeVector _x _returnvalue_3 0.0))
  (bind _returnvalue_5 (Math|Vector|SelectVector _returnvalue_4 _movementvector _collidingup))
  (bind (_x_2 _y_2) (Math|Vector|BreakVector _returnvalue_5))
  (bind _returnvalue_6 (Math|Float|Min(Float) _y_2 0.0))
  (bind _returnvalue_7 (Math|Vector|MakeVector _x_2 _returnvalue_6 0.0))
  (bind _returnvalue_8 (Math|Vector|SelectVector _returnvalue_7 _returnvalue_5 _collidingdown))
  ;[1 1 1] Movement Calculation
  (Physics|SetPhysicsLinearVelocity (Variables|Default|GetStaticMesh) _returnvalue_8 false "None") ; Input velocity calculated
  (switch Utilities|FlowControl|Switch|SwitchonBarType (Variables|Default|GetBarType) ; If Client Bar
    (:NewEnumerator0
      (Variables|Default|SetMovedLastPosition (Math|Vector|Equal(Vector) _returnvalue_2 (Variables|Default|GetLastKnownPosition) 0.1))
      (if (and (not (Variables|Default|GetMovedLastPosition)) (Math|Vector|Equal(Vector) _returnvalue_8 "0, 0, 0" 0.0001)) ; If bar is not moving and we have not reached an error threshold position from last known position
        (Transformation|SetActorLocation _returnvalue_2 true false) ; Re-sync the position
      ))))

(event EventBeginPlay
  ;[1 1 1] Set Material Only for Client's Real Bar (left bar)
  (Networking|SwitchHasAuthority
    (:Remote
      (switch Utilities|FlowControl|Switch|SwitchonBarType (Variables|Default|GetBarType)
        (:NewEnumerator0
          (Rendering|Material|SetMaterial (Variables|Default|GetStaticMesh) 0 "/Game/Materials/BasicGreen.BasicGreen")
          (Rendering|SetVisibility (Variables|Default|GetStaticMesh) false false))))))

(fn ConstructionScript)