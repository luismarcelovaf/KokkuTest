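; Client-side bar actor that moves along the Y axis through MoveUp, MoveDown and MoveStop events, which set a movement vector scaled by BarSpeed.
; Tick writes that vector to the static mesh as physics linear velocity, clamping Y to block movement past a touched boundary.
; Mesh overlaps with Boundary actors set and clear the up and down collision flags according to BoundaryType.
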(event OnComponentBeginOverlap(StaticMesh)
  (params (OverlappedComponent :type Primitive%20Component%20Object%20Reference) (OtherActor :type Actor%20Object%20Reference) (OtherComp :type Primitive%20Component%20Object%20Reference) (OtherBodyIndex :type Integer) (bFromSweep :type Boolean) (SweepResult :type Hit%20Result%20Structure%20%28by%20ref%29))
  ;[1 1 1] Start colliding
  (bind _asboundary (Utilities|Casting|CastToBoundary OtherActor))
  (switch Utilities|FlowControl|Switch|SwitchonBoundaryType (Variables|/Game/Blueprints/Actors/Boundary.Boundary_C|GetBoundaryType _asboundary)
    (:NewEnumerator0
      (Variables|Default|SetCollidingUp true))
    (:NewEnumerator1
      (Variables|Default|SetCollidingDown true))))

(event OnComponentEndOverlap(StaticMesh)
  (params (OverlappedComponent :type Primitive%20Component%20Object%20Reference) (OtherActor :type Actor%20Object%20Reference) (OtherComp :type Primitive%20Component%20Object%20Reference) (OtherBodyIndex :type Integer))
  ;[1 1 1] End colliding
  (bind _asboundary (Utilities|Casting|CastToBoundary OtherActor))
  (switch Utilities|FlowControl|Switch|SwitchonBoundaryType (Variables|/Game/Blueprints/Actors/Boundary.Boundary_C|GetBoundaryType _asboundary)
    (:NewEnumerator0
      (Variables|Default|SetCollidingUp false))
    (:NewEnumerator1
      (Variables|Default|SetCollidingDown false))))

(event Custom|MoveUp
  ;[1 1 1] Inputs
  (Variables|Default|SetMovementVector (* (Math|Vector|MakeVector 0.0 -1.0 0.0) (Variables|Default|GetBarSpeed))))

(event Custom|MoveDown
  ;[1 1 1] Inputs
  (Variables|Default|SetMovementVector (* (Math|Vector|MakeVector 0.0 1.0 0.0) (Variables|Default|GetBarSpeed))))

(event Custom|MoveStop
  ;[1 1 1] Inputs
  (Variables|Default|SetMovementVector "0, 0, 0"))

(event EventTick
  (params (DeltaSeconds :type Float%20%28single-precision%29))
  (bind _collidingup (Variables|Default|GetCollidingUp))
  (bind _movementvector (Variables|Default|GetMovementVector))
  (bind (_x _y) (Math|Vector|BreakVector _movementvector))
  (bind _returnvalue (Math|Float|Max(Float) _y 0.0))
  (bind _returnvalue_2 (Math|Vector|MakeVector _x _returnvalue 0.0))
  (bind _returnvalue_3 (Math|Vector|SelectVector _returnvalue_2 _movementvector _collidingup))
  (bind (_x_2 _y_2) (Math|Vector|BreakVector _returnvalue_3))
  ;[1 1 1] Movement Calculation
  (Physics|SetPhysicsLinearVelocity (Variables|Default|GetStaticMesh) (Math|Vector|SelectVector (Math|Vector|MakeVector _x_2 (Math|Float|Min(Float) _y_2 0.0) 0.0) _returnvalue_3 (Variables|Default|GetCollidingDown)) false "None"))

(fn ConstructionScript)