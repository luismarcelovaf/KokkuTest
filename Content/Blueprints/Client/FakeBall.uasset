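; Client-side stand-in ball for what appears to be a Pong-style game, smoothing the motion of a referenced RealBall.
; Each tick it interpolates toward RealBall and copies its velocity to the mesh's physics, or snaps to its position when too far away.
; Mesh overlaps predict bounces locally by mirroring Y velocity on a Boundary and X velocity on a Bar, zeroing Z.
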(event OnComponentBeginOverlap(StaticMesh)
  (params (OverlappedComponent :type Primitive%20Component%20Object%20Reference) (OtherActor :type Actor%20Object%20Reference) (OtherComp :type Primitive%20Component%20Object%20Reference) (OtherBodyIndex :type Integer) (bFromSweep :type Boolean) (SweepResult :type Hit%20Result%20Structure%20%28by%20ref%29))
  ;[1 1 1] Boundary Hit
  (Utilities|Casting|CastToBoundary OtherActor
    (:then
      (bind _returnvalue (Physics|GetPhysicsLinearVelocity (Variables|Default|GetStaticMesh) "None")) ; Hitting boundary does not change direction
      (Physics|SetPhysicsLinearVelocity (Variables|Default|GetStaticMesh) (Math|Vector|MakeVector (.X (Math|Vector|BreakVector _returnvalue)) (* (.Y (Math|Vector|BreakVector _returnvalue)) -1.0) 0.0) false "None"))
    (:CastFailed
      ;[1 1 1] Bar Hit
      (Utilities|Casting|CastToBar OtherActor)
      (bind _returnvalue_2 (Physics|GetPhysicsLinearVelocity (Variables|Default|GetStaticMesh) "None"))
      (Physics|SetPhysicsLinearVelocity (Variables|Default|GetStaticMesh) (Math|Vector|MakeVector (* (.X (Math|Vector|BreakVector _returnvalue_2)) -1.0) (.Y (Math|Vector|BreakVector _returnvalue_2)) 0.0) false "None"))))

(event EventTick
  (params (DeltaSeconds :type Float%20%28single-precision%29))
  (bind _returnvalue (Transformation|GetActorLocation))
  (bind _realball (Variables|Default|GetRealBall))
  (bind _returnvalue_2 (Transformation|GetActorLocation _realball))
  ;[1 1 1] Interpolates to real ball
  (if (> (Math|Vector|VectorLength (- _returnvalue _returnvalue_2)) 1e+03)
    (Transformation|SetActorLocation (Transformation|GetActorLocation (Variables|Default|GetRealBall)) false false)
    (else
      (Transformation|SetActorLocation (Math|Interpolation|VInterpTo _returnvalue _returnvalue_2 DeltaSeconds 2.0) false true)
      (Physics|SetPhysicsLinearVelocity (Variables|Default|GetStaticMesh) (Transformation|GetVelocity (Variables|Default|GetRealBall)) false "None"))))

(fn ConstructionScript)